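; Sample trigger-box actor that demonstrates the HorrorHand component on a Default_MovementCharacter.
; Box makes the right hand hold the Holdable on begin overlap, and Box1 swaps hands.
; Box2 releases both hands on begin overlap, while Box3 does the same on end overlap.
; Each handler casts the overlapping actor to the character and prints a debug string after the call.
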(event OnComponentBeginOverlap(Box)
  (params (OverlappedComponent :type Primitive%20Component%20Object%20Reference) (OtherActor :type Actor%20Object%20Reference) (OtherComp :type Primitive%20Component%20Object%20Reference) (OtherBodyIndex :type Integer) (bFromSweep :type Boolean) (SweepResult :type Hit%20Result%20Structure%20%28by%20ref%29))
  (bind _asdefault_movement_character (Utilities|Casting|CastToDefault_MovementCharacter OtherActor))
  (Class|HorrorHandComponent|Hold (Variables|/Game/Blueprints/Default_MovementCharacter.Default_MovementCharacter_C|GetHorrorHand _asdefault_movement_character) "RIGHT" (Variables|Default|GetHoldable))
  (Development|PrintString "HoldRight"))

(event OnComponentBeginOverlap(Box2)
  (params (OverlappedComponent :type Primitive%20Component%20Object%20Reference) (OtherActor :type Actor%20Object%20Reference) (OtherComp :type Primitive%20Component%20Object%20Reference) (OtherBodyIndex :type Integer) (bFromSweep :type Boolean) (SweepResult :type Hit%20Result%20Structure%20%28by%20ref%29))
  (bind _asdefault_movement_character (Utilities|Casting|CastToDefault_MovementCharacter OtherActor))
  (Class|HorrorHandComponent|Release (Variables|/Game/Blueprints/Default_MovementCharacter.Default_MovementCharacter_C|GetHorrorHand _asdefault_movement_character) "RIGHT")
  (Class|HorrorHandComponent|Release (Variables|/Game/Blueprints/Default_MovementCharacter.Default_MovementCharacter_C|GetHorrorHand _asdefault_movement_character) "LEFT")
  (Development|PrintString "Release All"))

(event OnComponentBeginOverlap(Box1)
  (params (OverlappedComponent :type Primitive%20Component%20Object%20Reference) (OtherActor :type Actor%20Object%20Reference) (OtherComp :type Primitive%20Component%20Object%20Reference) (OtherBodyIndex :type Integer) (bFromSweep :type Boolean) (SweepResult :type Hit%20Result%20Structure%20%28by%20ref%29))
  (bind _asdefault_movement_character (Utilities|Casting|CastToDefault_MovementCharacter OtherActor))
  (Class|HorrorHandComponent|Swap (Variables|/Game/Blueprints/Default_MovementCharacter.Default_MovementCharacter_C|GetHorrorHand _asdefault_movement_character))
  (Development|PrintString "Swap"))

(event OnComponentEndOverlap(Box3)
  (params (OverlappedComponent :type Primitive%20Component%20Object%20Reference) (OtherActor :type Actor%20Object%20Reference) (OtherComp :type Primitive%20Component%20Object%20Reference) (OtherBodyIndex :type Integer))
  (bind _asdefault_movement_character (Utilities|Casting|CastToDefault_MovementCharacter OtherActor))
  (Class|HorrorHandComponent|Release (Variables|/Game/Blueprints/Default_MovementCharacter.Default_MovementCharacter_C|GetHorrorHand _asdefault_movement_character) "RIGHT")
  (Class|HorrorHandComponent|Release (Variables|/Game/Blueprints/Default_MovementCharacter.Default_MovementCharacter_C|GetHorrorHand _asdefault_movement_character) "LEFT")
  (Development|PrintString "Release All"))

(event EventBeginPlay)

(event Collision|EventActorBeginOverlap
  (params (OtherActor :type Actor%20Object%20Reference)))

(event EventTick
  (params (DeltaSeconds :type Float%20%28single-precision%29)))

(fn ConstructionScript)