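; Player character for a horror game, handling camera-relative item pickup, basic movement and look input.
; Left click sphere-traces from the camera and, if the dominant hand is empty, has HorrorHand hold any valid HorrorHoldableInterface actor; Q releases the right hand, Space swaps.
; Tab toggles a UseSubCamera mode that shows the cursor and blocks look input, without switching cameras here.
; The HorrorEventCaller call is left unwired.
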(event Custom|HoldItem
  (bind _camera (Variables|Default|GetCamera))
  (bind _horrorhand (Variables|Default|GetHorrorHand))
  (bind _returnvalue (Transformation|GetWorldLocation _camera))
  (bind _handdominance (Variables|/Script/HorrorSystem.HorrorHandComponent|GetHandDominance _horrorhand))
  ;[1 1 1] HoldItem
  (bind (_outhit _returnvalue_2) (Collision|SphereTraceByChannel _returnvalue (+ _returnvalue (* (Math|Vector|GetForwardVector _camera) 1.5e+02)) 5.0 "TraceTypeQuery1" true 0 "ForDuration" true "(R=1.000000,G=0.000000,B=0.000000,A=1.000000)" "(R=0.000000,G=1.000000,B=0.000000,A=1.000000)" 0.5))
  (if _returnvalue_2
    (bind _returnvalue_3 (Class|HorrorHandComponent|IsEmptyHand _horrorhand _handdominance))
    (if _returnvalue_3
      (bind _ashorror_holdable_interface (Utilities|Casting|CastToHorrorHoldableInterface (.HitActor (Collision|BreakHitResult _outhit))))
      (if (Class|HorrorHoldableInterface|IsHoldable _ashorror_holdable_interface _horrorhand)
        (Class|HorrorHandComponent|Hold _horrorhand _handdominance _ashorror_holdable_interface)))))

(event Custom|SwapItem
  (Class|HorrorHandComponent|Swap (Variables|Default|GetHorrorHand)))

(event Custom|PutItem
  (Class|HorrorHandComponent|Release (Variables|Default|GetHorrorHand) "RIGHT"))

(event Input|AxisEvents|InputAxisMoveForward
  (params (AxisValue :type Float%20%28single-precision%29))
  ;[0 0.001123 0.08333] Movement Events
  (Pawn|Input|AddMovementInput (* (Math|Vector|GetForwardVector (Variables|Collision|GetCapsuleComponent)) AxisValue) 1.0 false))

(event Input|AxisEvents|InputAxisMoveRightward
  (params (AxisValue :type Float%20%28single-precision%29))
  ;[0 0.001123 0.08333] Movement Events
  (Pawn|Input|AddMovementInput (* (Math|Vector|GetRightVector (Variables|Collision|GetCapsuleComponent)) AxisValue) 1.0 false))

(event Input|AxisEvents|InputAxisTurnRight
  (params (AxisValue :type Float%20%28single-precision%29))
  ;[0 0.001123 0.08333] Movement Events
  (bind _asplayer_controller (Utilities|Casting|CastToPlayerController (Pawn|GetController)))
  (if (not (Variables|Default|GetUseSubCamera))
    (Class|PlayerController|AddYawInput _asplayer_controller AxisValue)))

(event Input|AxisEvents|InputAxisLookUp
  (params (AxisValue :type Float%20%28single-precision%29))
  ;[0 0.001123 0.08333] Movement Events
  (bind _asplayer_controller (Utilities|Casting|CastToPlayerController (Pawn|GetController)))
  (if (not (Variables|Default|GetUseSubCamera))
    (Class|PlayerController|AddPitchInput _asplayer_controller AxisValue)))

(event Input|KeyboardEvents|SpaceBar
  (params (Key :type Key%20Structure :default "None"))
  (:Pressed
    (CallFunction|SwapItem)))

(event Input|MouseEvents|LeftMouseButton
  (params (Key :type Key%20Structure :default "None"))
  (:Pressed
    (CallFunction|HoldItem)))

(event Input|KeyboardEvents|Tab
  (params (Key :type Key%20Structure :default "None"))
  (:Pressed
    (bind _asplayer_controller (Utilities|Casting|CastToPlayerController (Pawn|GetController)))
    (bind _output_get (Variables|Default|SetUseSubCamera (not (Variables|Default|GetUseSubCamera))))
    (if _output_get
      (Variables|/Script/Engine.PlayerController|SetbShowMouseCursor _asplayer_controller true)
      (else
        (Variables|/Script/Engine.PlayerController|SetbShowMouseCursor _asplayer_controller false)))))

(event Input|KeyboardEvents|Q
  (params (Key :type Key%20Structure :default "None"))
  (:Pressed
    (CallFunction|PutItem)))

(fn ConstructionScript)