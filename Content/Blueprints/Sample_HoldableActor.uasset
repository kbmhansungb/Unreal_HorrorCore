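; Sample holdable actor that a hand can pick up, move and put down through holdable and hand interface calls.
; While held, its Scene component is set or lerped toward the requested transform and its ActorSequence jumps to the end and stops.
; On release it teleports to the hand's put location, plays the sequence, and aligns its up vector to the hit normal (world up without a hit) with a hand-built shortest-arc quaternion.
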(event Custom|SetSequecne
  (params (PlayAnim :type Boolean))
  (bind _actorsequence (Variables|Default|GetActorSequence))
  (bind _sequenceplayer (Variables|/Script/ActorSequence.ActorSequenceComponent|GetSequencePlayer _actorsequence))
  (if PlayAnim
    (Sequencer|Player|Play _sequenceplayer :!class /Script/MovieScene.MovieSceneSequencePlayer)
    (else
      (Class|MovieSceneSequencePlayer|GotoEndandStop _sequenceplayer))))

(event EventBeginPlay)

(event Collision|EventActorBeginOverlap
  (params (OtherActor :type Actor%20Object%20Reference)))

(event EventLerpHoldableTransform
  (params (DesireTransform :type Transform%20%28by%20ref%29))
  (bind _scene (Variables|Default|GetScene))
  (Transformation|SetWorldTransform _scene (Math|Transform|Lerp(Transform) (Transformation|GetWorldTransform _scene) DesireTransform 0.2) false false))

(event EventResponseHoldHoldable
  (params (HandInterface :type Horror%20Hand%20Interface%20Interface%20%28by%20ref%29))
  (CallFunction|SetSequecne false))

(event EventResponseReleaseHoldable
  (params (HandInterface :type Horror%20Hand%20Interface%20Interface%20%28by%20ref%29))
  (bind _hitresult (Class|HorrorHandInterface|GetHoldablePutLocation HandInterface))
  (bind _returnvalue (Transformation|GetActorRotation))
  (bind _returnvalue_2 (Transformation|GetActorUpVector))
  (bind (_bblockinghit _binitialoverlap _time _distance _location _impactpoint _normal) (Collision|BreakHitResult _hitresult))
  (bind _returnvalue_3 (select _bblockinghit _normal "0, 0,1.000000"))
  (bind _returnvalue_4 (Math|Vector|CrossProduct _returnvalue_2 _returnvalue_3))
  (bind _returnvalue_5 (Math|Vector|DotProduct _returnvalue_2 _returnvalue_3))
  (bind _returnvalue_6 (Math|Vector|Normalize _returnvalue_4))
  (bind _returnvalue_7 (Math|Trig|Acos(Degrees) _returnvalue_5))
  (bind _returnvalue_8 (/ _returnvalue_7 2.0))
  (bind (_x _y _z) (Math|Vector|BreakVector _returnvalue_6))
  (bind _returnvalue_9 (Math|Trig|Sin(Radians) _returnvalue_8))
  (Transformation|SetActorLocation _location false true)
  (CallFunction|SetSequecne true)
  (Transformation|SetActorRotation (Class|KismetMathLibrary|QuatRotator (* (Utilities|Struct|MakeQuat (* _x _returnvalue_9) (* _y _returnvalue_9) (* _z _returnvalue_9) (Math|Trig|Cos(Radians) _returnvalue_8)) (Class|KismetMathLibrary|QuatMakefromEuler (Math|Vector|MakeVector (.roll _returnvalue) (.pitch _returnvalue) (.yaw _returnvalue))))) true))

(event EventSetHoldableTransform
  (params (DesireTransform :type Transform%20%28by%20ref%29))
  (Transformation|SetWorldTransform (Variables|Default|GetScene) DesireTransform false false))

(fn ConstructionScript)

(fn GetHoldableActor
  (return self))

(fn IsHoldable
  (params (HandInterface :type Horror%20Hand%20Interface%20Interface%20%28by%20ref%29))
  (return true))