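; HoldableItemActor is an item actor that a hand can hold, exposing itself and its HoldableItem through interface-style functions and always reporting as holdable.
; It positions its Scene component by composing RelativeTransform's relative transform, as a grip offset, with a desired transform.
; The move either snaps directly or blends from the current transform by a fixed alpha per call for smoothed following.
; Hold, release and response events are empty stubs.
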(event EventReleaseItemActor
  (params (HandComponent :type Horror%20Hand%20Component%20Object%20Reference)))

(event EventHoldItemActor
  (params (HandComponent :type Horror%20Hand%20Component%20Object%20Reference)))

(event EventSetHoldableTransform
  (params (DesireTransform :type Transform%20%28by%20ref%29))
  (Transformation|SetWorldTransform (Variables|Default|GetScene) (Math|Transform|ComposeTransforms (Transformation|GetRelativeTransform (Variables|Default|GetRelativeTransform)) DesireTransform) false false))

(event EventResponseReleaseHoldable
  (params (HandInterface :type Horror%20Hand%20Interface%20Interface%20%28by%20ref%29)))

(event EventResponseHoldHoldable
  (params (HandInterface :type Horror%20Hand%20Interface%20Interface%20%28by%20ref%29)))

(event EventLerpHoldableTransform
  (params (DesireTransform :type Transform%20%28by%20ref%29))
  (bind _scene (Variables|Default|GetScene))
  (Transformation|SetWorldTransform _scene (Math|Transform|Lerp(Transform) (Transformation|GetWorldTransform _scene) (Math|Transform|ComposeTransforms (Transformation|GetRelativeTransform (Variables|Default|GetRelativeTransform)) DesireTransform) 0.2) false false))

(fn ConstructionScript)

(fn GetHoldableActor
  (return self))

(fn GetItemInterface
  (return (LocalVariables|GetHoldableItem)))

(fn IsHoldable
  (params (HandInterface :type Horror%20Hand%20Interface%20Interface%20%28by%20ref%29))
  (return true))